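; Game instance Blueprint that fetches user account details from a web service and handles multiplayer session hosting and joining.
; Two near-identical events send GET requests built from URL, page and user key, differing in endpoint suffix, and store username, email, banned and remarks fields.
; HostGame creates a LAN session and opens the lobby as a listen server.
; JoinHost joins a supplied search result, printing success or failure.
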(event Custom|GetUserInfomationT
  (bind _result (Class|VaRestRequestJSON|ApplyURL (Class|VaRestRequestJSON|ConstructRequestExt "GET" "x_www_form_urlencoded_url") (Utilities|String|Append (Variables|Default|GetURL) (Variables|Default|GetInfoPage) "?rk=" (Variables|Default|GetUserKey) (Variables|Default|GetFName) "userinfoT")))
  (Variables|Default|SetUserName (Class|VaRestJsonValue|AsString (Class|VaRestJsonObject|GetField _result "username")))
  (Variables|Default|SetEmail (Class|VaRestJsonValue|AsString (Class|VaRestJsonObject|GetField _result "email")))
  (Variables|Default|SetBanned (Class|VaRestJsonValue|AsString (Class|VaRestJsonObject|GetField _result "banned")))
  (Variables|Default|SetRemarks (Class|VaRestJsonValue|AsString (Class|VaRestJsonObject|GetField _result "remarks"))))

(event Custom|HostGame
  ;[1 1 1] Can Make a Game
  (|Session (Game|GetPlayerController 0) 4 true
    (:OnSuccess
      (Game|OpenLevel(byName) "lobby" true "listen"))
    (:OnFailure
      (Development|PrintString "Didn't work"))))

(event Custom|JoinHost
  (params (Search%20Result :type Blueprint%20Session%20Result%20Structure))
  ;[1 1 1] Player Can Join Session
  (|JoinSession (Game|GetPlayerController 0) Search%20Result
    (:OnSuccess
      (Development|PrintString "Join Success"))
    (:OnFailure
      (Development|PrintString "Join fail"))))

(event Custom|GetUserInfomation
  (bind _result (Class|VaRestRequestJSON|ApplyURL (Class|VaRestRequestJSON|ConstructRequestExt "GET" "x_www_form_urlencoded_url") (Utilities|String|Append (Variables|Default|GetURL) (Variables|Default|GetInfoPage) "?rk=" (Variables|Default|GetUserKey) (Variables|Default|GetFName) "userinfo")))
  (Variables|Default|SetUserName (Class|VaRestJsonValue|AsString (Class|VaRestJsonObject|GetField _result "username")))
  (Variables|Default|SetEmail (Class|VaRestJsonValue|AsString (Class|VaRestJsonObject|GetField _result "email")))
  (Variables|Default|SetBanned (Class|VaRestJsonValue|AsString (Class|VaRestJsonObject|GetField _result "banned")))
  (Variables|Default|SetRemarks (Class|VaRestJsonValue|AsString (Class|VaRestJsonObject|GetField _result "remarks"))))